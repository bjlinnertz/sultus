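; Base character Blueprint for GAS-driven combat, with melee and ranged modes that switch camera and rotation behavior.
; BeginPlay grants initial and weapon abilities plus a regen effect; attack events activate abilities or confirm targeting.
; Sword overlaps with hostile characters and ADS-camera line traces send damage gameplay events to self, carrying the target.
; It also handles montage-timed death and knockback with hit stun, briefly removing ground friction and pawn collision.
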(event `MeleeAttack`
  ;[1 1 1] Any Abilities we use
  (if (`self.targeting`)
    (`AbilitySystemComponent.TargetConfirm` (`self.AbilitySystemComp`))
    (else
      (`AbilitySystemComponent.TryActivateAbilityByClass` (`self.AbilitySystemComp`) "/Game/Blueprints/Character/Weapons/MeleeAttack/GA_Melee.GA_Melee_C" true))))

(event `Switch Modes`
  ;[1 1 1] Switch weapons  modes
  (if (`self.RangedMode?`)
    (`self.MakeCameraControlRotation` true)
    (`KismetSystemLibrary.PrintString` "In Ranged Mode")
    (else
      (`self.MakeCameraControlRotation` false)
      (`KismetSystemLibrary.PrintString` "In Melee Mode"))))

(event `self.ReceiveBeginPlay`
  ;[1 1 1] Any Abilities we use
  (`self.AcquireAbilities` (`self.intial abilities`))
  (`self.AcquireAbilities` (`self.weapons`))
  (`AbilitySystemComponent.BP_ApplyGameplayEffectToSelf` :`self` (`self.AbilitySystemComp`) :`GameplayEffectClass` "/Game/Blueprints/Character/GameplayAbilities/GenralGameplayEffects/GE_BasicRegen.GE_BasicRegen_C"))

(event `Ranged Attack`
  ;[1 1 1] Any Abilities we use
  (if (`self.targeting`)
    (`AbilitySystemComponent.TargetConfirm` (`self.AbilitySystemComp`))
    (else
      (`AbilitySystemComponent.TryActivateAbilityByClass` (`self.AbilitySystemComp`) "/Game/Blueprints/Character/Weapons/RangeAttack/GA_RangeAttack.GA_RangeAttack_C" true)
      (`self.Firing`))))

(event `Firing`
  (bind _adscamera (`self.ADSCamera`))
  (bind _returnvalue (`SceneComponent.K2_GetComponentLocation` _adscamera))
  ;[1 1 1] Fire the Ranged Weapon
  (bind _outhit (`KismetSystemLibrary.LineTraceSingle` :`Start` _returnvalue :`End` (+ (* (`KismetMathLibrary.GetForwardVector` (`SceneComponent.K2_GetComponentRotation` _adscamera)) 2000.0) _returnvalue) :`TraceChannel` "TraceTypeQuery1" :`DrawDebugType` "Persistent"))
  (`AbilitySystemBlueprintLibrary.SendGameplayEventToActor` self (struct :`TagName` "weapon.sword.ranged.DealDamage") (make `GameplayEventData` (struct) null (`.HitActor` (`GameplayStatics.BreakHitResult` _outhit)))))

(event `MakeCameraControlRotation`
  (params (ShouldControlRotation :type Boolean))
  ;[1 1 1] Change camera depending on ranged vs. melee
  (if ShouldControlRotation
    (`ActorComponent.Activate` (`self.ADSCamera`) false)
    (`ActorComponent.Deactivate` (`self.Player Eye`))
    (set `self.bUseControllerRotationYaw` true)
    (set `CharacterMovementComponent.bOrientRotationToMovement` false (`self.CharacterMovement`))
    (else
      (`ActorComponent.Activate` (`self.Player Eye`) false)
      (`ActorComponent.Deactivate` (`self.ADSCamera`))
      (set `self.bUseControllerRotationYaw` false)
      (set `CharacterMovementComponent.bOrientRotationToMovement` true (`self.CharacterMovement`)))))

(event `self.SwordCollider.OnComponentBeginOverlap`
  (params (OverlappedComponent :type "PrimitiveComponent Object Reference") (OtherActor :type "Actor Object Reference") (OtherComp :type "PrimitiveComponent Object Reference") (OtherBodyIndex :type Integer) (bFromSweep :type Boolean) (SweepResult :type "HitResult Structure (by ref)"))
  ;[1 1 1] Collider for sword
  (if (!= OtherActor self)
    (bind _asbp_character_base (cast `/Game/Blueprints/Character/BP_Character_Base` OtherActor))
    (bind _returnvalue (`self.IsOtherHostile` _asbp_character_base self))
    (if _returnvalue
      (`AbilitySystemBlueprintLibrary.SendGameplayEventToActor` self (struct :`TagName` "skill.melee.DealDamage") (make `GameplayEventData` (struct) null OtherActor)))))

(event `self.BP_Die`
  ;[1 1 1] Die
  (bind _returnvalue (`self.PlayAnimMontage` "/Game/Blueprints/Character/Animations/AM_Die_Shinbi.AM_Die_Shinbi"))
  (`KismetSystemLibrary.Delay` _returnvalue)
  (`self.K2_DestroyActor`))

(event `PushCharacter`
  (params (ImpulseDirection :type "Vector Structure") (PushStrength :type "Float (double-precision)") (StunDuration :type "Float (double-precision)") (PushAnimation :type "AnimMontage Object Reference"))
  (bind _charactermovement (`self.CharacterMovement`))
  ;[1 1 1] Push character and hit stun
  (`self.Set Collision To Pawn` "ECR_Ignore")
  (`self.PlayAnimMontage` PushAnimation)
  (set `self.Default Ground Friction` (`CharacterMovementComponent.GroundFriction` _charactermovement))
  (set `CharacterMovementComponent.GroundFriction` 0.0 _charactermovement)
  (`CharacterMovementComponent.AddImpulse` (`self.CharacterMovement`) (* ImpulseDirection PushStrength) true)
  (if (> StunDuration 0.0)
    (`self.HitStun` StunDuration))
  (`KismetSystemLibrary.Delay` 0.3)
  (set `CharacterMovementComponent.GroundFriction` (`self.Default Ground Friction`) (`self.CharacterMovement`))
  (`self.Set Collision To Pawn` "ECR_Block"))

(fn `Set Collision To Pawn`
  (params (`New response` :type "ECollisionResponse Enum" :default "ECR_Ignore"))
  (`PrimitiveComponent.SetCollisionResponseToChannel` (`self.CapsuleComponent`) "ECC_Pawn" `New response`))

(fn `UserConstructionScript`)