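; Base Gameplay Ability Blueprint providing shared helper functions for character abilities, with activation and end events left as disabled stubs.
; A lookup casts the owning actor to the base character and player controller, feeding the other helpers.
; DoUICoolDown starts cooldowns on primary UI slots matching this ability's class.
; IsCostStillAvaliable compares Health or Quintessence against the negated ability cost, while Strength compares zero instead of its attribute.
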(fn `DoUICoolDown`
  (bind _playercontroller (`self.GetPlayerCharacterAndController`))
  (`/Engine/EditorBlueprintResources/StandardMacros.IsValid` _playercontroller
    (:`Is Valid`
      (for _array_element (`/Game/UI/WBP_PrimaryUI.Slots` (`/Game/Blueprints/Character/BP_PlayerController_Base.Primary UI` _playercontroller))
        (bind _returnvalue (`self.GetAbilityInfo`))
        (bind (_ability_info_cooldownduration _ability_info_cost _ability_info_costtype _ability_info_uimat _ability_info_abilityclass) (break `GameplayAbilityInfo` (`/Game/UI/WBP_Ability_Slot.Ability Info` _array_element)))
        (if (== _ability_info_abilityclass (`.AbilityClass` (break `GameplayAbilityInfo` _returnvalue)))
          (`/Game/UI/WBP_Ability_Slot.StartCoolDown` _array_element))))))

(fn `GetPlayerCharacterAndController`
  (returns (PlayerController :type "/Game/Blueprints/Character/BP_PlayerController_Base Object Reference") (`Character Base` :type "/Game/Blueprints/Character/BP_Character_Base Object Reference"))
  (bind _asbp_character_base (cast `/Game/Blueprints/Character/BP_Character_Base` (`self.GetOwningActorFromActorInfo`)))
  (bind _asbp_player_controller_base (cast `/Game/Blueprints/Character/BP_PlayerController_Base` (`Pawn.GetController` _asbp_character_base))
    (:`then`
      _)
    (:`CastFailed`
      _))
  (return _asbp_player_controller_base _asbp_character_base))

(fn `IsCostStillAvaliable`
  (returns (Can :type Boolean))
  (locals (cost :type "Float (double-precision)"))
  (bind _returnvalue (`self.GetAbilityInfo`))
  (set `local.cost` (* (`.Cost` (break `GameplayAbilityInfo` _returnvalue)) -1.0))
  (switch `EAbilityCostType` (`.CostType` (break `GameplayAbilityInfo` _returnvalue))
    (:`Health`
      (bind (_playercontroller _character_base) (`self.GetPlayerCharacterAndController`))
      (bind (_health_basevalue _health_currentvalue) (break `GameplayAttributeData` (`AttributeSet_Base.Health` (`Character_Base.AttributeSetBaseComp` _character_base))))
      (return (> _health_currentvalue (`local.cost`))))
    (:`Quintessence`
      (bind (_playercontroller_2 _character_base_2) (`self.GetPlayerCharacterAndController`))
      (bind (_quintessence_basevalue _quintessence_currentvalue) (break `GameplayAttributeData` (`AttributeSet_Base.Quintessence` (`Character_Base.AttributeSetBaseComp` _character_base_2))))
      (return (> _quintessence_currentvalue (`local.cost`))))
    (:`Strength`
      (bind (_playercontroller_3 _character_base_3) (`self.GetPlayerCharacterAndController`))
      (return (> 0.0 (`local.cost`))))))