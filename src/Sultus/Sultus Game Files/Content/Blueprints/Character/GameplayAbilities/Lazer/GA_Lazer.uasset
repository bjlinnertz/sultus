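; GA_Lazer is a Gameplay Ability that fires a channeled laser from the character during a casting montage.
; After a short delay it spawns BP_Lazer on the mesh's Lazer socket and enables camera-controlled rotation.
; Each DealDamage gameplay event applies damage and pushes hit characters away from the beam's end detector with stun, or ends the ability if cost is unavailable.
; Ending removes the draining cost effect, destroys the laser and disables camera-controlled rotation.
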(event `self.K2_ActivateAbility`
  (`GameplayAbility.K2_CommitAbility`)
  (`self.DoUICoolDown`)
  (`AbilityTask_PlayMontageAndWait.CreatePlayMontageAndWaitProxy` "None" "/Game/Blueprints/Character/Animations/AM_Lazer_Casting.AM_Lazer_Casting" 1.0 "None"
    (:`then`
      (`KismetSystemLibrary.Delay` 0.2)
      (bind (_playercontroller _character_base) (`self.GetPlayerCharacterAndController`))
      (bind (_asynctaskproxy _spawnedactor) (`AbilityTask_SpawnActor.SpawnActor` (struct) "/Game/Blueprints/Character/GameplayAbilities/Lazer/BP_Lazer.BP_Lazer_C" _character_base)
        (:`then`
          (bind _output_get (set `self.Lazer Actor` _spawnedactor))
          (`Actor.K2_AttachToComponent` _output_get (`Character.Mesh` _character_base) "Lazer" "SnapToTarget" "SnapToTarget" "KeepRelative" true)
          (`/Game/Blueprints/Character/BP_Character_Base.MakeCameraControlRotation` _character_base true)
          (bind (_asynctaskproxy_2 _payload) (`AbilityTask_WaitGameplayEvent.WaitGameplayEvent` (struct :`TagName` "skill.lazer.DealDamage") null)
            (:`EventReceived`
              (bind _can (`self.IsCostStillAvaliable`))
              (if _can
                (`GameplayAbility.BP_ApplyGameplayEffectToTarget` (`.TargetData` (break `GameplayEventData` _payload)) "/Game/Blueprints/Character/GameplayAbilities/Lazer/GE_Lazer_Damage.GE_Lazer_Damage_C")
                (for _array_element (`AbilitySystemBlueprintLibrary.GetActorsFromTargetData` (`.TargetData` (break `GameplayEventData` _payload)))
                  (bind _asbp_character_base (cast `/Game/Blueprints/Character/BP_Character_Base` _array_element))
                  (`/Game/Blueprints/Character/BP_Character_Base.PushCharacter` _asbp_character_base (`KismetMathLibrary.Normal` (- (`Actor.K2_GetActorLocation` _asbp_character_base) (`SceneComponent.K2_GetComponentLocation` (`/Game/Blueprints/Character/GameplayAbilities/Lazer/BP_Lazer.LazerEndDetector` (cast `/Game/Blueprints/Character/GameplayAbilities/Lazer/BP_Lazer` (`self.Lazer Actor`) :!pure true))))) 500.0 0.3 "/Game/Blueprints/Character/Animations/AM_HitStun.AM_HitStun"))
                (else
                  (`GameplayAbility.K2_EndAbility`))))))))
    (:`OnCompleted`
      (`GameplayAbility.K2_EndAbility` :!label _label))
    (:`OnBlendOut`
      (goto _label))
    (:`OnInterrupted`
      (goto _label))
    (:`OnCancelled`
      (goto _label))))

(event `self.K2_OnEndAbility`
  (params (bWasCancelled :type Boolean))
  (`GameplayAbility.BP_RemoveGameplayEffectFromOwnerWithAssetTags` (struct :`GameplayTags` (struct :`(TagName` "skill.lazer.drainingCost"))))
  (`Actor.K2_DestroyActor` (`self.Lazer Actor`))
  (bind (_playercontroller _character_base) (`self.GetPlayerCharacterAndController`))
  (`/Game/Blueprints/Character/BP_Character_Base.MakeCameraControlRotation` _character_base false))