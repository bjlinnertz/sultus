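; Laser beam actor for a character gameplay ability that tracks hostile characters touching its end detector.
; Each tick it stretches the skeletal beam by passing the detector's distance, minus the original length, to the AnimBP's end-bone offset.
; Detector overlaps maintain a hostile-filtered target list.
; A looping timer sends that list to the instigator as gameplay event target data for damage, even when empty.
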(event `self.ReceiveBeginPlay`
  ;[1 1 1] Send damage evet
  (set `self.Beam Original Legnth` (`KismetMathLibrary.VSize` (- (`SceneComponent.GetSocketLocation` (`self.SkeletalMesh`) "end") (`self.K2_GetActorLocation`))))
  (`KismetSystemLibrary.K2_SetTimerDelegate` (delegate `SendDealdamage`) 0.3 true))

(event `SendDealdamage`
  ;[1 1 1] Send damage evet
  (if (`KismetMathLibrary.Conv_IntToBool` (`KismetArrayLibrary.Array_Length` (`self.OverlapingActors`)))
    _
    (else
      _))
  (`AbilitySystemBlueprintLibrary.SendGameplayEventToActor` (`self.GetInstigator`) (struct) (make `GameplayEventData` (struct) null null null null (struct) (struct) (struct) 0.0 (`AbilitySystemBlueprintLibrary.AbilityTargetDataFromActorArray` (`self.OverlapingActors`)))))

(event `self.ReceiveTick`
  (params (DeltaSeconds :type "Float (single-precision)"))
  ;[1 1 1] Send damage evet
  (bind _asanim_bp_lazer_beam (cast `/Game/Blueprints/Character/GameplayAbilities/Lazer/Assests/AnimBP_LazerBeam` (`SkeletalMeshComponent.GetAnimInstance` (`self.SkeletalMesh`))))
  (set `/Game/Blueprints/Character/GameplayAbilities/Lazer/Assests/AnimBP_LazerBeam.end bone offest` (`KismetMathLibrary.MakeVector` (- (`KismetMathLibrary.VSize` (- (`SceneComponent.K2_GetComponentLocation` (`self.LazerEndDetector`)) (`self.K2_GetActorLocation`))) (`self.Beam Original Legnth`))) _asanim_bp_lazer_beam))

(event `self.LazerEndDetector.OnComponentBeginOverlap`
  (params (OverlappedComponent :type "PrimitiveComponent Object Reference") (OtherActor :type "Actor Object Reference") (OtherComp :type "PrimitiveComponent Object Reference") (OtherBodyIndex :type Integer) (bFromSweep :type Boolean) (SweepResult :type "HitResult Structure (by ref)"))
  (bind _asbp_character_base (cast `/Game/Blueprints/Character/BP_Character_Base` OtherActor))
  (bind _asbp_character_base_2 (cast `/Game/Blueprints/Character/BP_Character_Base` (`self.GetInstigator`)))
  (bind _returnvalue (`Character_Base.IsOtherHostile` _asbp_character_base_2 _asbp_character_base))
  (if _returnvalue
    (`KismetArrayLibrary.Array_AddUnique` (`self.OverlapingActors`) _asbp_character_base)))

(event `self.LazerEndDetector.OnComponentEndOverlap`
  (params (OverlappedComponent :type "PrimitiveComponent Object Reference") (OtherActor :type "Actor Object Reference") (OtherComp :type "PrimitiveComponent Object Reference") (OtherBodyIndex :type Integer))
  (bind _asbp_character_base (cast `/Game/Blueprints/Character/BP_Character_Base` OtherActor))
  (`KismetArrayLibrary.Array_RemoveItem` (`self.OverlapingActors`) _asbp_character_base))

(fn `UserConstructionScript`)