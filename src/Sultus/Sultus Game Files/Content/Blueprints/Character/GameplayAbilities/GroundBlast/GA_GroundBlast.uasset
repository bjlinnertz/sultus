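; Gameplay ability for Ground Blast, a player-targeted ground attack that damages and launches the characters it hits.
; After a cost check and targeting montage, it switches camera rotation mode and waits for user-confirmed data from a ground-select target actor.
; Confirmation commits the ability, starts the UI cooldown and plays the cast montage, spawning the blast effect, applying damage and pushing targets upward with a stun.
; Ending the ability restores the camera mode.
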(event `self.K2_ActivateAbility`
  (bind _can (`self.IsCostStillAvaliable`))
  (if _can
    (`AbilityTask_PlayMontageAndWait.CreatePlayMontageAndWaitProxy` "None" "/Game/Blueprints/Character/Animations/AM_GroundBlast_Targeting.AM_GroundBlast_Targeting"
      (:`then`
        (`KismetSystemLibrary.Delay` (`AnimSequenceBase.SequenceLength` (`self.GetCurrentMontage`)))
        (bind (_playercontroller _character_base) (`self.GetPlayerCharacterAndController`))
        (`/Game/Blueprints/Character/BP_Character_Base.MakeCameraControlRotation` _character_base true)
        (bind (_asynctaskproxy _data) (`AbilityTask_WaitTargetData.WaitTargetData` "None" "UserConfirmed" "/Game/Blueprints/Character/GameplayAbilities/GroundBlast/BP_GATargetActorGroundSelect.BP_GATargetActorGroundSelect_C" 200.0 (struct) (struct) null)
          (:`ValidData`
            (bind (_playercontroller_2 _character_base_2) (`self.GetPlayerCharacterAndController`))
            (set `/Game/Blueprints/Character/BP_Character_Base.targeting` true _character_base_2)
            (`self.K2_CommitAbility`)
            (`self.DoUICoolDown`)
            (`AbilityTask_PlayMontageAndWait.CreatePlayMontageAndWaitProxy` "None" "/Game/Blueprints/Character/Animations/AM_GroundBlast_Cast.AM_GroundBlast_Cast"
              (:`then`
                (`GameplayStatics.SpawnEmitterAtLocation` "/Game/Blueprints/Character/GameplayAbilities/GroundBlast/P_GroundBlast.P_GroundBlast" (`AbilitySystemBlueprintLibrary.GetTargetDataEndPoint` _data (- (`AbilitySystemBlueprintLibrary.GetDataCountFromTargetData` _data) 1)))
                (`self.BP_ApplyGameplayEffectToTarget` _data "/Game/Blueprints/Character/GameplayAbilities/GroundBlast/GE_GroundBlast_Damage.GE_GroundBlast_Damage_C")
                (for _array_element (`AbilitySystemBlueprintLibrary.GetActorsFromTargetData` _data)
                  (bind _asbp_character_base (cast `/Game/Blueprints/Character/BP_Character_Base` _array_element))
                  (`/Game/Blueprints/Character/BP_Character_Base.PushCharacter` _asbp_character_base (0.0 0.0 1.0) 500.0 2.0 "/Game/Blueprints/Character/Animations/AM_Die_Shinbi.AM_Die_Shinbi")
                  (`KismetSystemLibrary.Delay` 1.0)
                  (bind (_playercontroller_3 _character_base_3) (`self.GetPlayerCharacterAndController`))
                  (`/Game/Blueprints/Character/BP_Character_Base.MakeCameraControlRotation` _character_base_3 false)))
              (:`OnCompleted`
                (`self.K2_EndAbility` :!label _label))
              (:`OnBlendOut`
                (goto _label))
              (:`OnInterrupted`
                (goto _label))
              (:`OnCancelled`
                (goto _label))))
          (:`Cancelled`
            (`self.K2_EndAbility`)))))
    (else
      (`self.K2_EndAbility`))))

(event `self.K2_OnEndAbility`
  (params (bWasCancelled :type Boolean))
  (bind (_playercontroller _character_base) (`self.GetPlayerCharacterAndController`))
  (`/Game/Blueprints/Character/BP_Character_Base.MakeCameraControlRotation` _character_base false))