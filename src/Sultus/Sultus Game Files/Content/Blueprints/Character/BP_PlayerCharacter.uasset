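; BP_PlayerCharacter is the player character Blueprint that keeps the HUD's health and quintessence displays in sync with the character's stats.
; Its health and mana change events cast the controller to BP_PlayerController_Base and set the matching glass ball widget on PrimaryUI to the current-to-max ratio.
; BeginPlay, overlap, Tick and the construction script add no logic of their own.
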(event `self.BP_OnHealthChange`
  (params (Health :type "Float (single-precision)") (MaxHealth :type "Float (single-precision)"))
  (bind _asbp_player_controller_base (cast `/Game/Blueprints/Character/BP_PlayerController_Base` (`self.GetController`)))
  (`/Game/UI/WBP_GlassBall.SetPercentage` (`/Game/UI/WBP_PrimaryUI.Health_GlassBall` (`/Game/Blueprints/Character/BP_PlayerController_Base.Primary UI` _asbp_player_controller_base)) (/ Health MaxHealth)))

(event `self.BP_OnManaChange`
  (params (Quintessence :type "Float (single-precision)") (MaxQuintessence :type "Float (single-precision)"))
  (bind _asbp_player_controller_base (cast `/Game/Blueprints/Character/BP_PlayerController_Base` (`self.GetController`)))
  (`/Game/UI/WBP_GlassBall.SetPercentage` (`/Game/UI/WBP_PrimaryUI.Quintessence_GlassBall` (`/Game/Blueprints/Character/BP_PlayerController_Base.Primary UI` _asbp_player_controller_base)) (/ Quintessence MaxQuintessence)))

(fn `UserConstructionScript`
  (`parent.UserConstructionScript`))