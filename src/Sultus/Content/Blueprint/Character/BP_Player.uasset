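; BP_Player is a player character Blueprint that reacts to changes in Health and Quintessence.
; Its two change events each divide the current value by its maximum and print the ratio to screen, with no other gameplay response.
; BeginPlay, overlap and Tick are disabled placeholders, and the construction script only calls its parent.
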(event `self.BP_OnHealthChange`
  (params (Health :type "Float (single-precision)") (MaxHealth :type "Float (single-precision)"))
  (`KismetSystemLibrary.PrintString` (`KismetStringLibrary.Conv_DoubleToString` (/ Health MaxHealth))))

(event `self.BP_OnQuintessenceChange`
  (params (Quintessence :type "Float (single-precision)") (MaxQuintessence :type "Float (single-precision)"))
  (`KismetSystemLibrary.PrintString` (`KismetStringLibrary.Conv_DoubleToString` (/ Quintessence MaxQuintessence))))

(fn `UserConstructionScript`
  (`parent.UserConstructionScript`))