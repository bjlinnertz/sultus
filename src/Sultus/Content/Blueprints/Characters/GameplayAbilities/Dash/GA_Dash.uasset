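; GA_Dash is a gameplay ability that launches the owning character forward in a dash, damaging and knocking back targets.
; It commits, starts the UI cooldown, zeroes ground friction, adds a forward impulse and sets pawn collision to overlap while the dash montage plays.
; A dealDamage gameplay event applies the damage effect and pushes the target away with a stun.
; When the montage ends or is interrupted, friction and blocking collision are restored.
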(event `self.K2_ActivateAbility`
  (`self.K2_CommitAbility`)
  (`self.DoUICoolDown`)
  (bind _ascharacter (cast `Character` (`self.GetOwningActorFromActorInfo`))
    (:`then`
      (bind _charactermovement (`Character.CharacterMovement` _ascharacter))
      (set `self.OrigionalGroundFriction` (`CharacterMovementComponent.GroundFriction` _charactermovement))
      (set `CharacterMovementComponent.GroundFriction` 0.0 _charactermovement)
      (`CharacterMovementComponent.AddImpulse` _charactermovement (* (`Actor.GetActorForwardVector` _ascharacter) 2000.0) true)
      (bind _characterbase (`self.GetPlayerCharacterAndController`))
      (`/Game/Blueprints/Characters/BP_CharacterBase.SetCollisonToPawn` _characterbase "ECR_Overlap")
      (`AbilityTask_PlayMontageAndWait.CreatePlayMontageAndWaitProxy` "None" "/Game/Blueprints/Characters/Animation/AM_Dash_Shinbi.AM_Dash_Shinbi"
        (:`then`
          (bind (_asynctaskproxy _payload) (`AbilityTask_WaitGameplayEvent.WaitGameplayEvent` (struct :`TagName` "skill.dash.dealDamage") null)
            (:`EventReceived`
              (bind (_eventtag _instigator _target) (break `GameplayEventData` _payload))
              (`self.BP_ApplyGameplayEffectToTarget` (`AbilitySystemBlueprintLibrary.AbilityTargetDataFromActor` _target) "/Game/Blueprints/Characters/GameplayAbilities/Dash/GE_Dash_Damage.GE_Dash_Damage_C")
              (bind _asbp_character_base (cast `/Game/Blueprints/Characters/BP_CharacterBase` _target))
              (`/Game/Blueprints/Characters/BP_CharacterBase.PushCharacter` _asbp_character_base (`KismetMathLibrary.Normal` (- (`Actor.K2_GetActorLocation` _asbp_character_base) (`Actor.K2_GetActorLocation` (`self.GetOwningActorFromActorInfo`)))) 4000.0 5.0 null))))
        (:`OnCompleted`
          (set `CharacterMovementComponent.GroundFriction` (`self.OrigionalGroundFriction`) _charactermovement :!label _label)
          (bind _characterbase_2 (`self.GetPlayerCharacterAndController`))
          (`/Game/Blueprints/Characters/BP_CharacterBase.SetCollisonToPawn` _characterbase_2 "ECR_Block")
          (`self.K2_EndAbility`))
        (:`OnBlendOut`
          (goto _label))
        (:`OnInterrupted`
          (goto _label))
        (:`OnCancelled`
          (goto _label))))
    (:`CastFailed`
      (`self.K2_EndAbility`))))