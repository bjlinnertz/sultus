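; Gameplay ability that casts a lazer beam, damaging and knocking back targets while its cost remains affordable.
; Activation commits, plays the casting montage, then after a short delay attaches a spawned BP_Lazer to the mesh socket and changes the camera.
; Each damage gameplay event rechecks cost, then applies damage and pushes targets away from the beam's end detector, or ends the ability.
; Ending removes the draining cost effect, destroys the beam and reverts the camera.
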(event `self.K2_ActivateAbility`
  (`self.K2_CommitAbility`)
  (`self.DoUICoolDown`)
  (`AbilityTask_PlayMontageAndWait.CreatePlayMontageAndWaitProxy` "None" "/Game/Blueprints/Characters/Animation/AM_Lazer_Casting.AM_Lazer_Casting"
    (:`then`
      (`KismetSystemLibrary.Delay` 0.3)
      (bind _characterbase (`self.GetPlayerCharacterAndController`))
      (bind (_asynctaskproxy _spawnedactor) (`AbilityTask_SpawnActor.SpawnActor` (struct) "/Game/Blueprints/Characters/GameplayAbilities/Lazer/BP_Lazer.BP_Lazer_C" _characterbase)
        (:`then`
          (bind _output_get (set `self.LazerActor` _spawnedactor))
          (`Actor.K2_AttachToComponent` _output_get (`Character.Mesh` _characterbase) "Lazer" "SnapToTarget" "SnapToTarget" "KeepRelative" true)
          (`/Game/Blueprints/Characters/BP_CharacterBase.MakeCameraChange` _characterbase true)
          (bind (_asynctaskproxy_2 _payload) (`AbilityTask_WaitGameplayEvent.WaitGameplayEvent` (struct :`TagName` "skill.lazer.dealDamage") null)
            (:`EventReceived`
              (bind _can (`self.IsCostStillAvaliable`))
              (if _can
                (bind (_eventtag _instigator _target _optionalobject _optionalobject2 _contexthandle _instigatortags _targettags _eventmagnitude _targetdata) (break `GameplayEventData` _payload))
                (`self.BP_ApplyGameplayEffectToTarget` _targetdata "/Game/Blueprints/Characters/GameplayAbilities/Lazer/GE_Lazer_Damage.GE_Lazer_Damage_C")
                (for _array_element (`AbilitySystemBlueprintLibrary.GetActorsFromTargetData` _targetdata)
                  (bind _asbp_character_base (cast `/Game/Blueprints/Characters/BP_CharacterBase` _array_element))
                  (`/Game/Blueprints/Characters/BP_CharacterBase.PushCharacter` _asbp_character_base (`KismetMathLibrary.Normal` (- (`Actor.K2_GetActorLocation` _asbp_character_base) (`SceneComponent.K2_GetComponentLocation` (`/Game/Blueprints/Characters/GameplayAbilities/Lazer/BP_Lazer.LazerEndDetector` (cast `/Game/Blueprints/Characters/GameplayAbilities/Lazer/BP_Lazer` (`self.LazerActor`) :!pure true))))) 500.0 0.3 "/Game/Blueprints/Characters/Animation/AM_HitStun.AM_HitStun"))
                (else
                  (`self.K2_EndAbility`))))))))))

(event `self.K2_OnEndAbility`
  (params (bWasCancelled :type Boolean))
  (`self.BP_RemoveGameplayEffectFromOwnerWithAssetTags` (struct :`GameplayTags` (struct :`(TagName` "skill.lazer.drainingCost"))))
  (`Actor.K2_DestroyActor` (`self.LazerActor`))
  (bind _characterbase (`self.GetPlayerCharacterAndController`))
  (`/Game/Blueprints/Characters/BP_CharacterBase.MakeCameraChange` _characterbase false))