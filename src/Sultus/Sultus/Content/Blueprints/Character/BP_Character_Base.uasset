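; Base character Blueprint that uses the Gameplay Ability System for melee, dash and health regen.
; It grants the three abilities on BeginPlay and exposes events that activate each by class.
; Sword collider overlaps with other actors send itself a melee damage gameplay event carrying the target, with the hostility check left unwired.
; A generically named custom event plays the death montage, waits for its length, then destroys the actor.
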(event `Try HealthRegen`
  ;[1 1 1] Any Abilities we use
  (`AbilitySystemComponent.TryActivateAbilityByClass` (`self.AbilitySystemComp`) "/Game/Blueprints/Character/GameplayAbilities/HealthRegen/GA_HealthRegen.GA_HealthRegen_C" true))

(event `self.ReceiveBeginPlay`
  (`self.AcquireAbility` "/Game/Blueprints/Character/GameplayAbilities/Melee/GA_Melee.GA_Melee_C")
  (`self.AcquireAbility` "/Game/Blueprints/Character/GameplayAbilities/HealthRegen/GA_HealthRegen.GA_HealthRegen_C")
  (`self.AcquireAbility` "/Game/Blueprints/Character/GameplayAbilities/Dash/GA_Dash.GA_Dash_C"))

(event `MeleeAttack`
  ;[1 1 1] Any Abilities we use
  (`AbilitySystemComponent.TryActivateAbilityByClass` (`self.AbilitySystemComp`) "/Game/Blueprints/Character/GameplayAbilities/Melee/GA_Melee.GA_Melee_C" true))

(event `Try Dash Ability`
  ;[1 1 1] Any Abilities we use
  (`AbilitySystemComponent.TryActivateAbilityByClass` (`self.AbilitySystemComp`) "/Game/Blueprints/Character/GameplayAbilities/Dash/GA_Dash.GA_Dash_C" true))

(event `self.SwordCollider.OnComponentBeginOverlap`
  (params (OverlappedComponent :type "PrimitiveComponent Object Reference") (OtherActor :type "Actor Object Reference") (OtherComp :type "PrimitiveComponent Object Reference") (OtherBodyIndex :type Integer) (bFromSweep :type Boolean) (SweepResult :type "HitResult Structure (by ref)"))
  (if (!= OtherActor self)
    (`AbilitySystemBlueprintLibrary.SendGameplayEventToActor` self (struct :`TagName` "skill.melee.DealDamage") (make `GameplayEventData` (struct) null OtherActor))))

(event `CustomEvent`
  (bind _returnvalue (`self.PlayAnimMontage` "/Game/Blueprints/Character/Animations/AM_Die_Shinbi.AM_Die_Shinbi"))
  (`KismetSystemLibrary.Delay` _returnvalue)
  (`self.K2_DestroyActor`))

(fn `UserConstructionScript`)